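; CustomCharacter is a player character Blueprint with input handlers for camera look, jumping and movement.
; Turn and LookUp call controller yaw and pitch input with a constant zero, not the axis value, and Jump triggers on press.
; MoveForward and MoveRight scale forward and right vectors by axis value, from a rotator that puts actor yaw into roll, leaving pitch and yaw zero.
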(event `InputAxis|Turn`
  (params (AxisValue :type "Float (single-precision)"))
  ;[1 1 1] 플레이어 카메라 동작
  (`self.AddControllerYawInput` 0.0))

(event `InputAction|Jump`
  (params (Key :type "Key Structure" :default "AnyKey"))
  ;[1 1 1] 점프
  (:`Pressed`
    (`self.Jump`)))

(event `InputAxis|LookUp`
  (params (AxisValue :type "Float (single-precision)"))
  ;[1 1 1] 플레이어 카메라 동작
  (`self.AddControllerPitchInput` 0.0))

(event `InputAxis|MoveForward`
  (params (AxisValue :type "Float (single-precision)"))
  ;[1 1 1] 이동구현
  (`self.AddMovementInput` (`KismetMathLibrary.GetForwardVector` (`KismetMathLibrary.MakeRotator` (.yaw (`self.K2_GetActorRotation`)))) AxisValue))

(event `InputAxis|MoveRight`
  (params (AxisValue :type "Float (single-precision)"))
  ;[1 1 1] 이동구현
  (`self.AddMovementInput` (`KismetMathLibrary.GetRightVector` (`KismetMathLibrary.MakeRotator` (.yaw (`self.K2_GetActorRotation`)))) AxisValue))

(fn `UserConstructionScript`)